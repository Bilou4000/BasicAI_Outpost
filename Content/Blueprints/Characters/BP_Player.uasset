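; BP_Player is the player character Blueprint, adding a smooth aim-down-sights transition.
; The aim event plays a timeline whose alpha blends the camera's field of view between base and aiming values and slides the weapon's relative Y position between its hip and aimed locations.
; Stopping aim reverses the same timeline, so the transition eases back from its current point.
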(event `Aim_1`
  (bind _weapon (`self.Weapon`))
  (bind (_relativelocation_x _relativelocation_y _relativelocation_z) (`KismetMathLibrary.BreakVector` (`SceneComponent.RelativeLocation` _weapon)))
  ;[1 1 1] Smooth FOV when aiming
  (bind (_direction _aimingtimeline) (`Timeline|SmoothAim` :!label _label)
    (:`Update`
      (`CameraComponent.SetFieldOfView` (`self.Camera`) (`KismetMathLibrary.Lerp` (`self.BaseFOV`) (`self.AimingFOV`) _aimingtimeline))
      (`SceneComponent.K2_SetRelativeLocation` _weapon (`KismetMathLibrary.MakeVector` _relativelocation_x (`KismetMathLibrary.Lerp` (`self.BaseWeaponLocation`) (`self.AimingWeaponLocation`) _aimingtimeline) _relativelocation_z) false false))))

(event `StopAiming_1`
  ;[1 1 1] Smooth FOV when aiming
  (goto _label :!via `Reverse`))

(fn `UserConstructionScript`
  (`parent.UserConstructionScript`))