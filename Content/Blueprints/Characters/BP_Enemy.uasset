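; BP_Enemy is an enemy character Blueprint that extends its parent's shooting behavior with damage dealing.
; Its Shoot event waits for the cooldown delay, calls the parent Shoot, then applies damage to the hit actor if it is valid and not tagged as Ally.
; The construction script only calls the parent's.
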(event `self.Shoot`
  (params (Start :type "Vector Structure") (End :type "Vector Structure"))
  (bind (_bblockinghit _binitialoverlap _time _distance _location _impactpoint _normal _impactnormal _physmat _hitactor) (`GameplayStatics.BreakHitResult` (`self.ShootHit`)))
  (`KismetSystemLibrary.Delay` (`self.ShootCooldown`))
  (`parent.Shoot` Start End)
  (`/Engine/EditorBlueprintResources/StandardMacros.IsValid` _hitactor
    (:`Is Valid`
      (if (not (`self.ActorHasTag` _hitactor "Ally"))
        (`GameplayStatics.ApplyDamage` _hitactor (`self.Damages`))))))

(fn `UserConstructionScript`
  (`parent.UserConstructionScript`))