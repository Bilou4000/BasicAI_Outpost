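; BP_Isaac is the player character, able to shoot, aim and direct a BP_Ally companion's targeting.
; Shoot passes a camera-forward trace to the parent, emits hearing noise and damages hit actors not tagged Ally.
; Each such hit actor is written to the ally AI's blackboard as its target, using the ally found at BeginPlay.
; Aiming plays a timeline that blends camera FOV and weapon position, reversed on release.
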(event `self.ReceiveBeginPlay`
  (`parent.ReceiveBeginPlay`)
  (bind _returnvalue (`GameplayStatics.GetActorOfClass` "/Game/Blueprints/Characters/Ally/BP_Ally.BP_Ally_C"))
  (set `self.Bp Ally` _returnvalue))

(event `self.Shoot`
  (params (Start :type "Vector Structure") (End :type "Vector Structure"))
  (bind _returnvalue (`GameplayStatics.GetPlayerCameraManager` 0))
  (bind (_bblockinghit _binitialoverlap _time _distance _location _impactpoint _normal _impactnormal _physmat _hitactor) (`GameplayStatics.BreakHitResult` (`self.ShootHit`)))
  (bind _returnvalue_2 (`PlayerCameraManager.GetCameraLocation` _returnvalue))
  ;[1 1 1] Plyaer Shoot
  (`parent.Shoot` _returnvalue_2 (+ _returnvalue_2 (* (`KismetMathLibrary.GetForwardVector` (`PlayerCameraManager.GetCameraRotation` _returnvalue)) (`self.ShootRange`))))
  (`self.MakeNoise` 1.0 self (`self.K2_GetActorLocation`) 0.0 "Hearing")
  (if _bblockinghit
    (if (not (`self.ActorHasTag` _hitactor "Ally"))
      (`GameplayStatics.ApplyDamage` _hitactor (`self.Damages`))
      (`BlackboardComponent.SetValueAsObject` (`AIBlueprintHelperLibrary.GetBlackboard` (`AIBlueprintHelperLibrary.GetAIController` (`self.Bp Ally`))) (`self.TargetRefKey`) _hitactor))))

(event `Aim_1`
  (bind _weapon (`self.Weapon`))
  (bind (_relativelocation_x _relativelocation_y _relativelocation_z) (`KismetMathLibrary.BreakVector` (`SceneComponent.RelativeLocation` _weapon)))
  ;[1 1 1] Smooth FOV when aiming
  (bind (_direction _aimingtimeline) (`Timeline|Timeline` :!label _label)
    (:`Update`
      (`CameraComponent.SetFieldOfView` (`self.Camera`) (`KismetMathLibrary.Lerp` (`self.BaseFOV`) (`self.AimingFOV`) _aimingtimeline))
      (`SceneComponent.K2_SetRelativeLocation` _weapon (`KismetMathLibrary.MakeVector` _relativelocation_x (`KismetMathLibrary.Lerp` (`self.BaseWeaponLocation`) (`self.AimingWeaponLocation`) _aimingtimeline) _relativelocation_z) false false))))

(event `StopAiming_1`
  ;[1 1 1] Smooth FOV when aiming
  (goto _label :!via `Reverse`))

(fn `UserConstructionScript`
  (`parent.UserConstructionScript`))