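; BP_Grenade is a timed grenade actor that explodes and deals radial damage.
; On BeginPlay it waits for TimeBeforeExplosion, then applies damage with falloff around its Sphere component, ignoring every actor of ClassToIgnore.
; It draws a debug sphere at the outer damage radius and then destroys itself.
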(event `self.ReceiveBeginPlay`
  (bind _damage_outer_radius (`self.Damage Outer Radius`))
  (bind _returnvalue (`SceneComponent.K2_GetComponentLocation` (`self.Sphere`)))
  ;[1 1 1] Grenade explodes + deal damage
  (`KismetSystemLibrary.Delay` (`self.timeBeforeExplosion`))
  (bind _outactors (`GameplayStatics.GetAllActorsOfClass` (`self.classToIgnore`)))
  (`GameplayStatics.ApplyRadialDamageWithFalloff` (`self.damages`) (`self.minimumDamages`) _returnvalue (`self.Damage Inner Radius`) _damage_outer_radius (`self.Damage Falloff`) null _outactors self null)
  (`KismetSystemLibrary.DrawDebugSphere` _returnvalue _damage_outer_radius 12 (struct :`R` 1.0 :`B` 0.00697 :`A` 1.0) 5.0 2.0)
  (`self.K2_DestroyActor`))

(fn `UserConstructionScript`)